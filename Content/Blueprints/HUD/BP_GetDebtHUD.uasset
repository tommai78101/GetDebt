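; HUD Blueprint that creates and removes the game's main menu, in-game overlay, game over, intro and credits widgets.
; BeginPlay caches the MainPlayerController as widget owner for paired Create and Delete functions.
; Creation skips already valid widgets except credits, which always builds anew, while deletion only removes from parent without clearing references.
; Deleting the intro also hides the mouse cursor, and state-based visibility logic sits unconnected.
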(event EventBeginPlay
  (bind _asmain_player_controller (Utilities|Casting|CastToMainPlayerController (Game|GetPlayerController 0)))
  (Variables|Default|SetPlayerController _asmain_player_controller))

(event EventActorBeginOverlap
  (params (OtherActor :type Actor%20Object%20Reference)))

(event EventTick
  (params (DeltaSeconds :type Float%20%28single-precision%29)))

(fn ConstructionScript)

(fn CreateMainMenu
  (if (not (Utilities|IsValid (Variables|Default|GetMainMenuWidget)))
    (bind _returnvalue (UserInterface|CreateWidget "/Game/Blueprints/HUD/MainMenuWidget.MainMenuWidget_C" (Variables|Default|GetPlayerController)))
    (bind _output_get (Variables|Default|SetMainMenuWidget _returnvalue))
    (UserInterface|Viewport|AddtoViewport _output_get 0)))

(fn DeleteMainMenu
  (bind _mainmenuwidget (Variables|Default|GetMainMenuWidget))
  (if (Utilities|IsValid _mainmenuwidget)
    (Widget|RemovefromParent _mainmenuwidget)))

(fn CreateinGameOverlay
  (if (not (Utilities|IsValid (Variables|Default|GetGameOverlayWidget)))
    (bind _returnvalue (UserInterface|CreateWidget "/Game/Blueprints/HUD/GameOverlayWidget.GameOverlayWidget_C" (Variables|Default|GetPlayerController)))
    (bind _output_get (Variables|Default|SetGameOverlayWidget _returnvalue))
    (UserInterface|Viewport|AddtoViewport _output_get 0)))

(fn DeleteinGameOverlay
  (bind _gameoverlaywidget (Variables|Default|GetGameOverlayWidget))
  (if (Utilities|IsValid _gameoverlaywidget)
    (Widget|RemovefromParent _gameoverlaywidget)))

(fn CreateGameOver
  (if (not (Utilities|IsValid (Variables|Default|GetGameOverWidget)))
    (bind _returnvalue (UserInterface|CreateWidget "/Game/Blueprints/HUD/GameOverWidget.GameOverWidget_C" (Variables|Default|GetPlayerController)))
    (bind _output_get (Variables|Default|SetGameOverWidget _returnvalue))
    (UserInterface|Viewport|AddtoViewport _output_get 0)))

(fn DeleteGameOver
  (bind _gameoverwidget (Variables|Default|GetGameOverWidget))
  (if (Utilities|IsValid _gameoverwidget)
    (Widget|RemovefromParent _gameoverwidget)))

(fn CreateIntro
  (if (not (Utilities|IsValid (Variables|Default|GetIntroWidget)))
    (bind _returnvalue (UserInterface|CreateWidget "/Game/Blueprints/HUD/IntroWidget.IntroWidget_C" (Variables|Default|GetPlayerController)))
    (bind _output_get (Variables|Default|SetIntroWidget _returnvalue))
    (UserInterface|Viewport|AddtoViewport _output_get 0)))

(fn DeleteIntro
  (bind _introwidget (Variables|Default|GetIntroWidget))
  (if (Utilities|IsValid _introwidget)
    (Widget|RemovefromParent _introwidget)
    (Variables|/Script/Engine.PlayerController|SetbShowMouseCursor (Game|GetPlayerController 0) false)))

(fn CreateCredits
  (bind _returnvalue (UserInterface|CreateWidget "/Game/Blueprints/HUD/CreditsWidget.CreditsWidget_C" (Variables|Default|GetPlayerController)))
  (bind _output_get (Variables|Default|SetCreditsWidget _returnvalue))
  (UserInterface|Viewport|AddtoViewport _output_get 0))

(fn DeleteCredits
  (bind _creditswidget (Variables|Default|GetCreditsWidget))
  (if (Utilities|IsValid _creditswidget)
    (Widget|RemovefromParent _creditswidget)))